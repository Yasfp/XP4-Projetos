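; BP_ItemJogavel is a throwable distraction item that emits a noise event when it hits something.
; The first Sphere component hit reports a loud AI noise at the actor's location with itself as instigator, gated by an un-reset DoOnce.
; Pegar handles pickup by calling Destruir, which destroys the actor after a short delay, and returning the static mesh asset.
; PegarItem only prints a debug string.
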(event OnComponentHit(Sphere)
  (params (HitComponent :type Primitive%20Component%20Object%20Reference) (OtherActor :type Actor%20Object%20Reference) (OtherComp :type Primitive%20Component%20Object%20Reference) (NormalImpulse :type Vector :default "0, 0, 0") (Hit :type Hit%20Result%20Structure%20%28by%20ref%29))
  (Utilities|FlowControl|DoOnce false
    (:Completed
      (Class|AISenseHearing|ReportNoiseEvent (Transformation|GetActorLocation) 5e+02 self 0.0 "None")
      (Development|PrintString "Barulho"))))

(event Custom|Destruir
  (Utilities|FlowControl|Delay 0.2)
  (Actor|DestroyActor))

(fn ConstructionScript)

(fn PegarItem
  (Development|PrintString "Pegou")
  (return 0))

(fn Pegar
  (CallFunction|Destruir)
  (return (Variables|/Script/Engine.StaticMeshComponent|GetStaticMesh (Variables|Default|GetStaticMesh))))