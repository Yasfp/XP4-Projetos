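; BP_DogAI is the enemy dog entity, with an attack that knocks the third-person player into the air.
; Atacar sphere-traces for Pawns far along the capsule's forward vector and launches any BP_ThirdPersonCharacter it hits.
; The launch uses a fixed world-space velocity, sideways and upward, regardless of the dog's facing.
; The event graph and construction script are empty, so nothing here calls Atacar.
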(event EventBeginPlay)

(fn ConstructionScript)

(fn Atacar
  (bind _self self)
  (bind _capsulecomponent (Variables|Collision|GetCapsuleComponent _self))
  (bind _returnvalue (Transformation|GetWorldLocation _capsulecomponent))
  (bind _outhit (Collision|SphereTraceForObjects _returnvalue (+ (* (Math|Vector|GetForwardVector (Transformation|GetWorldRotation _capsulecomponent)) 1e+04) _returnvalue) 0.0 (Utilities|Array|MakeArray "ObjectTypeQuery3") false 0 "None"))
  (if true
    (bind _asbp_third_person_character (Utilities|Casting|CastToBP_ThirdPersonCharacter (.HitActor (Collision|BreakHitResult _outhit))))
    (Character|LaunchCharacter _asbp_third_person_character "0.0,1300.0,800.0" false false)))