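; BP_NPC is a friendly NPC Blueprint that shows dialogue lines on screen.
; Each Falar (talk) call sets the Interrompido (interrupted) Blackboard key, then after a brief delay advances through the Dialogos array.
; It creates a WBP_CaixaDialogo widget when needed to display the current line, removing it shortly after the index passes the end.
; The Interrompido event and Pegar function are empty stubs.
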(event Custom|Interrompido)

(event EventFalar
  ;[0.15 0.15 0.15 0.5] Dialogos
  ;[0.15 0.15 0.15 0.5] Seta Bool Interrompido (Blackboard
  (Utilities|FlowControl|Sequence
    (:then_0
      (AI|Components|Blackboard|SetValueasBool (AI|GetBlackboard 0) (Utilities|Name|MakeLiteralName "Interrompido") true))
    (:then_1
      (Utilities|FlowControl|Delay 0.1)
      (Math|Integer|IncrementInt (Variables|Default|GetIndex)
        (:%20%20
          (if (< (Variables|Default|GetIndex) (Utilities|Array|Length (Variables|Default|GetDialogos)))
            (Variables|Default|GetUI
              (:then
                _)
              (:else
                (bind _returnvalue (UserInterface|CreateWidget "/Game/Dynamic/Widgets/WBP_CaixaDialogo.WBP_CaixaDialogo_C" (Game|GetPlayerController 0)))
                (bind _output_get (Variables|Default|SetUI _returnvalue))
                (UserInterface|Viewport|AddtoViewport _output_get 0)))
            (Rendering|Components|TextRender|SetText (Variables|/Game/Dynamic/Widgets/WBP_CaixaDialogo.WBP_CaixaDialogo_C|GetTalkText (Variables|Default|GetUI)) (Utilities|Text|ToText(String) (Utilities|Array|Get(acopy) (Variables|Default|GetDialogos) (Variables|Default|GetIndex))))
            (else
              (Utilities|FlowControl|Delay 1.0)
              (Widget|RemovefromParent (Variables|Default|GetUI)))))))))

(fn ConstructionScript)

(fn Pegar
  (return 0))