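; GM_Main is the game mode that deals random cards from its ItemDataGM pool to the third-person character.
; AdicionarCarta, gated by PodeAdicionar, loops over the player's ItemDataP, and non-matching entries trigger printing the card's DataTable description and moving it to the player.
; Tick calls the character's VerificarCartas every frame.
; VerificarPrimeiraVez, uncalled here, removes a "Debug" placeholder card from the player.
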(event Custom|ChamarFunçãoAdd
  (CallFunction|AdicionarCarta))

(event EventTick
  (params (DeltaSeconds :type Float%20%28single-precision%29))
  (bind _asbp_third_person_character (Utilities|Casting|CastToBP_ThirdPersonCharacter (Game|GetPlayerCharacter 0)))
  (Default|VerificarCartas _asbp_third_person_character))

(fn ConstructionScript)

(fn AdicionarCarta
  (bind _item_data_gm (Variables|Default|GetItem%20Data%20GM))
  (Variables|Default|SetCarta%20Alea (.OutItem (Utilities|Array|Random _item_data_gm)))
  (if (Variables|Default|GetPode%20Adicionar)
    (bind _returnvalue (Actor|GetActorOfClass "/Game/Dynamic/Blueprints/Player/BP_ThirdPersonCharacter.BP_ThirdPersonCharacter_C"))
    (for _array_element (Variables|/Game/Dynamic/Blueprints/Player/BP_ThirdPersonCharacter.BP_ThirdPersonCharacter_C|GetItem%20data%20P _returnvalue)
      (if (not (== (.rowname (Utilities|Struct|BreakS_Slots _array_element)) (.rowname (Utilities|Struct|BreakS_Slots (Variables|Default|GetCarta%20Alea)))))
        (|DarDescrição (.datatable (Utilities|Struct|BreakS_Slots (Variables|Default|GetCarta%20Alea))) (.rowname (Utilities|Struct|BreakS_Slots (Variables|Default|GetCarta%20Alea))))
        (Utilities|Array|Add (Variables|/Game/Dynamic/Blueprints/Player/BP_ThirdPersonCharacter.BP_ThirdPersonCharacter_C|GetItem%20data%20P _returnvalue) (Variables|Default|GetCarta%20Alea))
        (Utilities|Array|RemoveItem _item_data_gm (Variables|Default|GetCarta%20Alea))
        (Variables|Default|SetPode%20Adicionar false)))))

(fn VerificarPrimeiraVez
  (bind _asbp_third_person_character (Utilities|Casting|CastToBP_ThirdPersonCharacter (Game|GetPlayerCharacter 0)))
  (if (Utilities|Array|ContainsItem (Variables|/Game/Dynamic/Blueprints/Player/BP_ThirdPersonCharacter.BP_ThirdPersonCharacter_C|GetItem%20data%20P _asbp_third_person_character) (Utilities|Struct|MakeS_Slots (Utilities|Struct|MakeDataTableRowHandle "/Game/Dynamic/Assets/Cartas/Data/DB_Cartas.DB_Cartas" "Debug")))
    (Utilities|Array|RemoveItem (Variables|/Game/Dynamic/Blueprints/Player/BP_ThirdPersonCharacter.BP_ThirdPersonCharacter_C|GetItem%20data%20P _asbp_third_person_character) (Utilities|Struct|MakeS_Slots (Utilities|Struct|MakeDataTableRowHandle "/Game/Dynamic/Assets/Cartas/Data/DB_Cartas.DB_Cartas" "Debug")))
    (Development|PrintString "Foi!")))