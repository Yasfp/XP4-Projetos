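; BP_GhostTrail is an actor meant to leave a fading afterimage of the player, but its logic is disconnected and BeginPlay does nothing.
; The unwired chain gives a PoseableMesh the player's skeletal mesh, the M_GhostTrail material and a random parameter, then copies the current pose as a snapshot.
; A Timeline would then drive the material's Alpha and destroy the actor when it finishes.
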(event EventBeginPlay)

(fn ConstructionScript)