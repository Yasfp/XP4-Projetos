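; BP_Dog is an enemy dog that wanders and chases pawns it sees.
; A looping random walk moves it to navigable points within a radius, pausing after each successful move.
; Unless Distraido (distracted) is set, PawnSensing sightings raise its speed and start a chase; a retriggerable delay then restores walking speed and wandering.
; A state check picks between wandering and an empty Esconder (hide) event, but nothing here calls it.
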(event OnSeePawn(PawnSensing)
  (params (Pawn :type Pawn%20Object%20Reference))
  (if (not (Variables|Default|GetDistraido))
    (Development|PrintString "Hello")
    (Variables|/Script/Engine.CharacterMovementComponent|SetMaxWalkSpeed (Variables|Character|GetCharacterMovement) 4e+02)
    (AI|AIMoveTo self "0, 0, 0" Pawn 5.0 false
      (:then
        (Utilities|FlowControl|RetriggerableDelay 2.0)
        (Variables|/Script/Engine.CharacterMovementComponent|SetMaxWalkSpeed (Variables|Character|GetCharacterMovement) 175.0)
        (Development|PrintString "Beyyyy")
        (CallFunction|RamdomWalk)))))

(event Custom|Ramdom_Walk
  (bind _randomlocation (Class|NavigationSystemV1|GetRandomLocationinNavigableRadius (Transformation|GetActorLocation) 1e+03 0 0))
  (AI|AIMoveTo self _randomlocation 0 5.0 false
    (:OnSuccess
      (Utilities|FlowControl|Delay 4.0)
      (CallFunction|RamdomWalk))))

(event Custom|Verificação%20de%20estado
  (if (Variables|Default|GetDistraido)
    (CallFunction|Esconder)
    (else
      (CallFunction|RamdomWalk))))

(event Custom|Esconder)

(event EventBeginPlay
  (CallFunction|RamdomWalk))

(fn ConstructionScript)